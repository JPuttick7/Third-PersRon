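; MyCharacter is a character Blueprint that handles HUD setup and end-of-game screens for a horde game mode.
; BeginPlay adds a crosshair and two instances of the same health indicator widget to the viewport.
; Tick polls HordeGameMode, creating game-over and win or lose widgets on every frame the flags are set, then quits after a delay.
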(event EventBeginPlay
  (Utilities|FlowControl|Sequence
    (:then_0
      (bind _returnvalue (UserInterface|CreateWidget "/Game/UI/WBP_Crosshair.WBP_Crosshair_C"))
      (UserInterface|Viewport|AddtoViewport _returnvalue 0))
    (:then_1
      (bind _returnvalue_2 (UserInterface|CreateWidget "/Game/UI/WBP_HealthIndicator.WBP_HealthIndicator_C"))
      (UserInterface|Viewport|AddtoViewport _returnvalue_2 0))
    (:then_2
      (bind _returnvalue_3 (UserInterface|CreateWidget "/Game/UI/WBP_HealthIndicator.WBP_HealthIndicator_C"))
      (UserInterface|Viewport|AddtoViewport _returnvalue_3 0))))

(event EventTick
  (params (DeltaSeconds :type Float%20%28single-precision%29))
  (bind _ashorde_game_mode (Utilities|Casting|CastToHordeGameMode (Game|GetGameMode)))
  (if (Variables|/Script/thirdpersron.HordeGameMode|GetbGameOver _ashorde_game_mode)
    (Utilities|FlowControl|Sequence
      (:then_0
        (bind _returnvalue (UserInterface|CreateWidget "/Game/UI/GAMEOVER.GAMEOVER_C"))
        (UserInterface|Viewport|AddtoViewport _returnvalue 0))
      (:then_1
        (if (Variables|/Script/thirdpersron.HordeGameMode|GetbWin _ashorde_game_mode)
          (bind _returnvalue_2 (UserInterface|CreateWidget "/Game/UI/YOUWIN.YOUWIN_C"))
          (UserInterface|Viewport|AddtoViewport _returnvalue_2 0)
          (Utilities|FlowControl|Delay 5.0)
          (Game|QuitGame 0 "Quit" true)
          (elif (Variables|/Script/thirdpersron.HordeGameMode|GetbLose _ashorde_game_mode)
            (bind _returnvalue_3 (UserInterface|CreateWidget "/Game/UI/YOULOSE.YOULOSE_C"))
            (UserInterface|Viewport|AddtoViewport _returnvalue_3 0)
            (Utilities|FlowControl|Delay 5.0)
            (Game|QuitGame 0 "Quit" true)))))))

(fn ConstructionScript)